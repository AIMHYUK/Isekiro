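; Trigger-volume actor that switches a referenced wire spot's state as actors enter and leave its Box.
; Begin overlap calls EnableWireSpot(false) on WireSpotActor and end overlap calls it with true, each guarded by a validity check.
; Neither event filters the overlapping actor or counts overlaps.
; Both print debug strings, with "enable" shown on the false call.
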(event `self.Box.OnComponentBeginOverlap`
  (params (OverlappedComponent :type "PrimitiveComponent Object Reference") (OtherActor :type "Actor Object Reference") (OtherComp :type "PrimitiveComponent Object Reference") (OtherBodyIndex :type Integer) (bFromSweep :type Boolean) (SweepResult :type "HitResult Structure (by ref)"))
  (`/Engine/EditorBlueprintResources/StandardMacros.IsValid` (`self.WireSpotActor`)
    (:`Is Valid`
      (`/Game/BluePrintsPlayer/BP_Actor.EnableWireSpot` (`self.WireSpotActor`) false)
      (`KismetSystemLibrary.PrintString` "enable"))))

(event `self.Box.OnComponentEndOverlap`
  (params (OverlappedComponent :type "PrimitiveComponent Object Reference") (OtherActor :type "Actor Object Reference") (OtherComp :type "PrimitiveComponent Object Reference") (OtherBodyIndex :type Integer))
  (`/Engine/EditorBlueprintResources/StandardMacros.IsValid` (`self.WireSpotActor`)
    (:`Is Valid`
      (`/Game/BluePrintsPlayer/BP_Actor.EnableWireSpot` (`self.WireSpotActor`) true)
      (`KismetSystemLibrary.PrintString` "disableenable"))))

(fn `UserConstructionScript`)