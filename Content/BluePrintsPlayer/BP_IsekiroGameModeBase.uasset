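; Game mode for Isekiro that handles level intros, background audio and fade-driven travel between the main menu and two game worlds.
; BeginPlay locks input, plays the level's track and fades in through WBP_Fade, whose finish callback restores input or opens the next level in the cycle.
; StartupFight locks hero input and starts the fade-out.
; SetupActorTransform teleports an actor to BP_HeroPlayerStart, rotated along the horizontal boss axis.
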(event `self.ReceiveBeginPlay`
  (bind _returnvalue (`GameplayStatics.GetPlayerController` 0))
  (`Controller.SetIgnoreLookInput` _returnvalue true)
  (`Controller.SetIgnoreMoveInput` _returnvalue true)
  (bind _returnvalue_2 (`|CreateWidget` "/Game/BluePrintsPlayer/WBP_Fade.WBP_Fade_C" (`GameplayStatics.GetPlayerController` 0)))
  (bind _output_get (set `self.FadeWIdget` _returnvalue_2))
  (add `/Game/BluePrintsPlayer/WBP_Fade.OnFadeFinished` _output_get (delegate `CustomEvent`))
  (`UserWidget.AddToViewport` _output_get 10)
  (`/Game/BluePrintsPlayer/WBP_Fade.StartFadeIn` _output_get)
  (bind _returnvalue_3 (`GameplayStatics.GetCurrentLevelName` true))
  (switch `string` _returnvalue_3
    (:`MainMap`
      (`self.PlayBackgroundAudio` "MAINMENU"))
    (:`GameWorld`
      (`self.PlayBackgroundAudio` "ASHINACASTLE"))
    (:`GameWorld1`
      (`self.PlayBackgroundAudio` "GENICHIRO"))))

(event `CustomEvent`
  (params (bFadeOut :type Boolean))
  (bind _returnvalue (`GameplayStatics.GetPlayerController` 0))
  (if bFadeOut
    (bind _returnvalue_2 (`GameplayStatics.GetCurrentLevelName` true))
    (switch `string` _returnvalue_2
      (:`MainMap`
        (`GameplayStatics.OpenLevel` "GameWorld"))
      (:`GameWorld`
        (`GameplayStatics.OpenLevel` "GameWorld1"))
      (:`GameWorld1`
        (`GameplayStatics.OpenLevel` "MainMap")))
    (else
      (`Controller.ResetIgnoreLookInput` _returnvalue)
      (`Controller.ResetIgnoreMoveInput` _returnvalue))))

(event `BPStartFadeOut`
  (bind _fadewidget (`self.FadeWIdget`))
  (if (not (`Widget.IsInViewport` _fadewidget))
    (`UserWidget.AddToViewport` _fadewidget 0))
  (`self.FadeOutBackgroundAudio` 1.6)
  (`/Game/BluePrintsPlayer/WBP_Fade.StartFadeOut` (`self.FadeWIdget`)))

(event `BPStartFadeIn`
  (`/Game/BluePrintsPlayer/WBP_Fade.StartFadeIn` (`self.FadeWIdget`)))

(fn `SetupActorTransform`
  (params (Actor :type "/Game/BluePrintsPlayer/BP_MyHeroCharacter Object Reference") (Transform :type "Transform Structure"))
  (`|ExecutionSequence`
    (:`then_0`
      (bind _returnvalue (`GameplayStatics.GetActorOfClass` "/Game/BluePrintsPlayer/BP_HeroPlayerStart.BP_HeroPlayerStart_C"))
      (bind _returnvalue_2 (`self.GetTransform` _returnvalue))
      (`KismetSystemLibrary.PrintString` (`KismetStringLibrary.Conv_TransformToString` _returnvalue_2))
      (`self.K2_SetActorTransform` (`local.Actor`) _returnvalue_2 false true))
    (:`then_1`
      (bind _returnvalue_3 (`GameplayStatics.GetActorOfClass` "/Game/Blueprints/Boss/BP_BossTest3.BP_BossTest3_C"))
      (bind (_returnvalue_x _returnvalue_y) (`KismetMathLibrary.BreakVector` (`self.K2_GetActorLocation` _returnvalue_3)))
      (bind (_returnvalue_x_2 _returnvalue_y_2 _returnvalue_z) (`KismetMathLibrary.BreakVector` (`self.K2_GetActorLocation` _returnvalue)))
      (`self.K2_SetActorRotation` (`local.Actor`) (`KismetMathLibrary.Conv_VectorToRotator` (`KismetMathLibrary.GetDirectionUnitVector` (- (`KismetMathLibrary.MakeVector` _returnvalue_x _returnvalue_y _returnvalue_z) (`KismetMathLibrary.MakeVector` _returnvalue_x_2 _returnvalue_y_2 _returnvalue_z)))) true))))

(fn `StartupFight`
  (params (Actor :type "Actor Object Reference"))
  (bind _asbp_my_hero_character (cast `/Game/BluePrintsPlayer/BP_MyHeroCharacter` Actor))
  (bind _returnvalue (`Pawn.GetController` _asbp_my_hero_character))
  (`Controller.SetIgnoreMoveInput` _returnvalue true)
  (`Controller.SetIgnoreLookInput` _returnvalue true)
  (`self.SetActorEnableCollision` false)
  (`self.BPStartFadeOut`))

(fn `UserConstructionScript`)