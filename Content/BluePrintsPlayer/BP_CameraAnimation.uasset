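; BP_CameraAnimation is an actor that plays a gameplay camera animation on the first player controller and takes over that player's view.
; PlayCameraAnim starts the animation through the Gameplay Cameras subsystem, stores the handle and switches the view target to itself.
; EndCameraAnimation stops that handle non-immediately, returns the view to the player character and destroys the actor after a short delay.
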(event `PlayCameraAnim`
  (bind _returnvalue (`GameplayStatics.GetPlayerController` 0))
  (bind _returnvalue_2 (`GameplayCamerasSubsystem.PlayCameraAnimation` :`self` (subsystem `GameplayCamerasSubsystem`) :`PlayerController` _returnvalue))
  (`PlayerController.SetViewTargetWithBlend` _returnvalue self 0.0 "VTBlend_Linear" 0.0 false))

(event `EndCameraAnimation`
  (`GameplayCamerasSubsystem.StopCameraAnimation` (subsystem `GameplayCamerasSubsystem`) (`GameplayStatics.GetPlayerController` 0) (stale `PlayCameraAnim` _returnvalue_2) false)
  (`PlayerController.SetViewTargetWithBlend` (`GameplayStatics.GetPlayerController` 0) (`GameplayStatics.GetPlayerCharacter` 0) 0.0 "VTBlend_Linear" 0.0 false)
  (`KismetSystemLibrary.Delay` 0.1)
  (`self.K2_DestroyActor` self))

(fn `UserConstructionScript`)